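; Paper2D runner character that constantly moves along +X and gains speed when the player alternates left and right power inputs.
; Each valid tap raises MaxWalkSpeed, scaled by a speed-based curve and capped at MaxSpeed, while Tick bleeds it off through a second curve.
; Tick also picks the idle or run flipbook, scales run playback to velocity and plays footstep sounds on frames 1 and 5.
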(event Input|EnhancedActionEvents|EnhancedInputActionIA_PowerLeft
  (params (ActionValue :type Boolean) (ElapsedSeconds :type Float%20%28double-precision%29) (TriggeredSeconds :type Float%20%28double-precision%29) (InputAction :type Input%20Action%20Object%20Reference :default "/Game/Input/Actions/IA_PowerLeft.IA_PowerLeft"))
  (:Started
    (switch Utilities|FlowControl|Switch|SwitchonE_Input (Variables|Default|GetLastInput)
      (:NewEnumerator0
        _)
      (:NewEnumerator2
        _))
    (CallFunction|IncreaseSpeed)
    (Variables|Default|SetLastInput "NewEnumerator1")))

(event Input|EnhancedActionEvents|EnhancedInputActionIA_PowerRight
  (params (ActionValue :type Boolean) (ElapsedSeconds :type Float%20%28double-precision%29) (TriggeredSeconds :type Float%20%28double-precision%29) (InputAction :type Input%20Action%20Object%20Reference :default "/Game/Input/Actions/IA_PowerRight.IA_PowerRight"))
  (:Started
    (switch Utilities|FlowControl|Switch|SwitchonE_Input (Variables|Default|GetLastInput)
      (:NewEnumerator0
        _)
      (:NewEnumerator1
        _))
    (CallFunction|IncreaseSpeed)
    (Variables|Default|SetLastInput "NewEnumerator2")))

(event EventBeginPlay
  (bind _asplayer_controller (Utilities|Casting|CastToPlayerController (Pawn|GetController)))
  (Input|AddMappingContext (PlayerController|LocalPlayerSubsystems|GetEnhancedInputLocalPlayerSubsystem _asplayer_controller) "/Game/Input/IMC_Runner.IMC_Runner" 0 "(bIgnoreAllPressedKeysUntilRelease=True,bForceImmediately=False,bNotifyUserSettings=False)"))

(event Collision|EventActorBeginOverlap
  (params (OtherActor :type Actor%20Object%20Reference)))

(event EventTick
  (params (DeltaSeconds :type Float%20%28single-precision%29))
  (bind _sprite (Variables|Default|GetSprite))
  (bind _returnvalue (Class|PaperFlipbookComponent|GetPlaybackPositioninFrames _sprite))
  (Pawn|Input|AddMovementInput "1.000000,0.000000,0.000000" 1.0 false)
  (bind _returnvalue_2 (CallFunction|DecreaseSpeed))
  (Sprite|SetFlipbook (Variables|Default|GetSprite) _returnvalue_2)
  (if (== (Class|PaperFlipbookComponent|GetFlipbook (Variables|Default|GetSprite)) "/Game/PaperAssets/Mash_Runner_Assets/Runner/FB_Runner_Run.FB_Runner_Run")
    (Components|Timeline|SetPlayRate (Variables|Default|GetSprite) (/ (Math|Vector|VectorLength (Variables|/Script/Engine.MovementComponent|GetVelocity (Variables|Character|GetCharacterMovement))) (Variables|Default|GetMaxSpeed)))
    (if (or (== _returnvalue 1) (== _returnvalue 5))
      (Utilities|FlowControl|DoOnce false :!label _label
        (:Completed
          (Audio|PlaySound2D "/Game/Sounds/Cue_Footstep.Cue_Footstep" 1.0 1.0 0.0 0 0)))
      (else
        (goto _label Reset)))
    (else
      (Components|Timeline|SetPlayRate (Variables|Default|GetSprite) 1.0))))

(fn ConstructionScript)

(fn IncreaseSpeed
  (Variables|/Script/Engine.CharacterMovementComponent|SetMaxWalkSpeed (Variables|Character|GetCharacterMovement) (Math|Float|Clamp(Float) (+ (Variables|/Script/Engine.CharacterMovementComponent|GetMaxWalkSpeed (Variables|Character|GetCharacterMovement)) (* (Variables|Default|GetSprintIncreasedOnTap) (Math|Curves|GetFloatValue (Variables|Default|GetSpeedIncreaseRamp) (Math|Vector|VectorLength (Variables|/Script/Engine.MovementComponent|GetVelocity (Variables|Character|GetCharacterMovement)))))) 0.0 (Variables|Default|GetMaxSpeed))))

(fn DecreaseSpeed
  (Variables|/Script/Engine.CharacterMovementComponent|SetMaxWalkSpeed (Variables|Character|GetCharacterMovement) (Math|Float|Max(Float) (- (Variables|/Script/Engine.CharacterMovementComponent|GetMaxWalkSpeed (Variables|Character|GetCharacterMovement)) (* (Utilities|Time|GetWorldDeltaSeconds) (* (Variables|Default|GetSlowMultiplier) (Math|Curves|GetFloatValue (Variables|Default|GetSpeedDecreaseRamp) (Math|Vector|VectorLength (Variables|/Script/Engine.MovementComponent|GetVelocity (Variables|Character|GetCharacterMovement))))))) 0.0))
  (return (select (> (Math|Vector|VectorLength (Variables|/Script/Engine.MovementComponent|GetVelocity (Variables|Character|GetCharacterMovement))) 0.0) "/Game/PaperAssets/Mash_Runner_Assets/Runner/FB_Runner_Run.FB_Runner_Run" "/Game/PaperAssets/Mash_Runner_Assets/Runner/FB_Runner_Idle.FB_Runner_Idle")))