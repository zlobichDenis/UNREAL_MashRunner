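; AI controller that plays a BP_Runner by faking alternating left and right power inputs.
; On possess it caches the runner, and from BeginPlay it starts a one-shot timer with a random delay between minimum and maximum input delays.
; A FlipFlop in SimulateInput switches between the runner's left and right power calls, then re-arms the timer, producing an irregular, self-renewing input rhythm.
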(event Custom|SimulateInput
  (Utilities|FlowControl|FlipFlop
    (:A
      (Default|SimulatePowerLeft (Variables|Default|GetOwningRunner)))
    (:B
      (Default|SimulatePowerRight (Variables|Default|GetOwningRunner))))
  (CallFunction|SimulateInputwithDelay))

(event EventBeginPlay
  (CallFunction|SimulateInputwithDelay))

(event EventTick
  (params (DeltaSeconds :type Float%20%28single-precision%29)))

(event EventPossess
  (params (PossessedPawn :type Pawn%20Object%20Reference))
  (bind _asbp_runner (Utilities|Casting|CastToBP_Runner PossessedPawn))
  (Variables|Default|SetOwningRunner _asbp_runner))

(fn ConstructionScript)

(fn SimulateInputwithDelay
  (Utilities|Time|SetTimerbyEvent (EventDispatchers|CreateEvent :!event Custom|SimulateInput) (Math|Random|RandomFloatinRange (Variables|Default|GetMinInputDelay) (Variables|Default|GetMaxInputDelay))))