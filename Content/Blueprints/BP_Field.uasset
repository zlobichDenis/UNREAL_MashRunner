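; BP_Field is a 2D Paper2D stage that builds its layout from a configurable part count and part length.
; The construction script adds one field sprite component per part, tiled along X.
; Helper functions stretch and center the top and bottom boxes across the whole length, keeping their other axes.
; Both goals are offset along X by the position of the last part, relative to their existing location.
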(event EventBeginPlay)

(event Collision|EventActorBeginOverlap
  (params (OtherActor :type Actor%20Object%20Reference)))

(event EventTick
  (params (DeltaSeconds :type Float%20%28single-precision%29)))

(fn ConstructionScript
  (for _index (range 0 (- (Variables|Default|GetStageParts) 1))
    (bind _returnvalue (AddComponent|AddPaperSpriteComponent false (Math|Transform|MakeTransform (Math|Vector|MakeVector (Math|Conversions|ToFloat(Integer) (* _index (Variables|Default|GetStageLength))) 0.0 0.0) "0, 0, 0" "1.000000,1.000000,1.000000")))
    (Rendering|Components|Sprite|SetSprite _returnvalue "/Game/PaperAssets/Mash_Runner_Assets/Background/T_Field_Sprite.T_Field_Sprite"))
  (CallFunction|UpdateBoxExtent (Variables|Default|GetBoxTOp))
  (CallFunction|UpdateBoxExtent (Variables|Default|GetBoxBottom))
  (CallFunction|SetRelativeLocation (Variables|Default|GetBoxTOp))
  (CallFunction|SetRelativeLocation (Variables|Default|GetBoxBottom))
  (CallFunction|SetGoalLocation (Variables|Default|GetGoalTop))
  (CallFunction|SetGoalLocation (Variables|Default|GetGoalBottom)))

(fn UpdateBoxExtent
  (params (Box :type Box%20Component%20Object%20Reference))
  (bind _boxextent (Variables|/Script/Engine.BoxComponent|GetBoxExtent Box))
  (Components|Box|SetBoxExtent Box (Math|Vector|MakeVector (Math|Conversions|ToFloat(Integer) (* (/ (Variables|Default|GetStageLength) 2) (Variables|Default|GetStageParts))) (.y _boxextent) (.z _boxextent)) true))

(fn SetRelativeLocation
  (params (Box :type Box%20Component%20Object%20Reference))
  (bind _relativelocation (Variables|/Script/Engine.SceneComponent|GetRelativeLocation Box))
  (Transformation|SetRelativeLocation Box (Math|Vector|MakeVector (Math|Conversions|ToFloat(Integer) (- (/ (* (Variables|Default|GetStageLength) (Variables|Default|GetStageParts)) 2) (/ (Variables|Default|GetStageLength) 2))) (.y _relativelocation) (.z _relativelocation)) false false))

(fn SetGoalLocation
  (params (Goal :type Scene%20Component%20Object%20Reference))
  (bind _relativelocation (Variables|/Script/Engine.SceneComponent|GetRelativeLocation Goal))
  (Transformation|SetRelativeLocation Goal (Math|Vector|MakeVector (+ (* (- (Variables|Default|GetStageParts) 1) (Variables|Default|GetStageLength)) (.x _relativelocation)) (.y _relativelocation) (.z _relativelocation)) false false))